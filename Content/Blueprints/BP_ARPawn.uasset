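; AR player pawn that adds the BP_Menu widget on begin play and lets a screen tap reposition the scene's BP_SpawnSceneActor.
; A tap first runs WorldHitTest, a deprojected line trace against scene objects.
; If that hits nothing, an AR tracked-object trace, excluding feature points and ground plane, supplies the position from its first result.
; The existing actor is moved there (the call is duplicated) and the coordinates are printed.
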(event `self.ReceiveBeginPlay`
  (bind _returnvalue (`|CreateWidget` "/Game/Blueprints/UI/BP_Menu.BP_Menu_C" (`GameplayStatics.GetPlayerController` 0)))
  (`UserWidget.AddToViewport` _returnvalue 0))

(event `InputTouch`
  (params (Location :type "Vector Structure") (FingerIndex :type "ETouchIndex Enum"))
  (bind (_locationx _locationy) (`PlayerController.GetInputTouchState` (`GameplayStatics.GetPlayerController` 0) "Touch1"))
  (bind _returnvalue (`KismetMathLibrary.MakeVector2D` _locationx _locationy))
  (:`Pressed`
    (bind (_outhit _returnvalue_2) (`self.WorldHitTest` _returnvalue))
    (if (not _returnvalue_2)
      (bind _returnvalue_3 (`ARBlueprintLibrary.LineTraceTrackedObjects` _returnvalue false false))
      (`/Engine/EditorBlueprintResources/StandardMacros.CompareInt` (`KismetArrayLibrary.Array_Length` _returnvalue_3)
        (:`>`
          (bind _returnvalue_4 (`GameplayStatics.GetActorOfClass` "/Game/Blueprints/BP_SpawnSceneActor.BP_SpawnSceneActor_C"))
          (bind _location (.location (`ARTraceResultLibrary.GetLocalToWorldTransform` (`|GetArrayItem` _returnvalue_3))))
          (`KismetSystemLibrary.PrintString` (`KismetTextLibrary.Conv_TextToString` (`|FormatText` "Poner en {x} {y} {z}" (.x _location) (.y _location) (.z _location))))
          (`self.K2_SetActorLocation` _returnvalue_4 _location false false)
          (bind _returnvalue_5 (`GameplayStatics.GetActorOfClass` "/Game/Blueprints/BP_SpawnSceneActor.BP_SpawnSceneActor_C"))
          (`self.K2_SetActorLocation` _returnvalue_5 _location false false))))))

(fn `UserConstructionScript`)

(fn `WorldHitTest`
  (params (ScreenPosition :type "Vector2D Structure"))
  (returns (OutHit :type "HitResult Structure") (ReturnValue :type Boolean))
  (bind (_worldposition _worlddirection) (`GameplayStatics.DeprojectScreenToWorld` (`GameplayStatics.GetPlayerController` 0) ScreenPosition))
  (bind (_outhit _returnvalue) (`KismetSystemLibrary.LineTraceSingleForObjects` _worldposition (+ _worldposition (* _worlddirection 1000.0)) (`|MakeArray` "ObjectTypeQuery1" "ObjectTypeQuery2" "ObjectTypeQuery3" "ObjectTypeQuery4" "ObjectTypeQuery5" "ObjectTypeQuery6" :!type "EObjectTypeQuery Enum")))
  (return _outhit _returnvalue))